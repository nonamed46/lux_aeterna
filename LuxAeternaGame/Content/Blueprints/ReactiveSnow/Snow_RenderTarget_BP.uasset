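; Reactive snow capture actor that follows the player and maintains a persistent render target of the snow.
; BeginPlay clears both render targets and passes the capture's ortho width to SnowMPC.
; Each tick, it moves by pixel-grid-snapped steps toward the player and publishes its location to SnowMPC.
; It then draws a dynamic material into the persistent target, offset by that move so accumulated data scrolls with the capture.
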(event `self.ReceiveBeginPlay`
  (`|ExecutionSequence`
    (:`then_0`
      (`KismetMaterialLibrary.SetScalarParameterValue` "/Game/Blueprints/ReactiveSnow/SnowMPC.SnowMPC" "Size" (`SceneCaptureComponent2D.OrthoWidth` (`self.SceneCaptureComponent2D`)))
      (bind _returnvalue (`KismetMaterialLibrary.CreateDynamicMaterialInstance` "/Game/Blueprints/ReactiveSnow/SnowDrawToPersistent.SnowDrawToPersistent"))
      (set `self.DrawToPMat` _returnvalue)
      (`KismetRenderingLibrary.ClearRenderTarget2D` "/Game/Blueprints/ReactiveSnow/SnowRenderTarget.SnowRenderTarget")
      (`KismetRenderingLibrary.ClearRenderTarget2D` "/Game/Blueprints/ReactiveSnow/RenderTargetPersistent.RenderTargetPersistent"))))

(event `MoveRT`
  (bind (_returnvalue_x _returnvalue_y) (`KismetMathLibrary.BreakVector` (`self.K2_GetActorLocation` (`GameplayStatics.GetPlayerCharacter` 0))))
  (bind (_returnvalue_x_2 _returnvalue_y_2) (`KismetMathLibrary.BreakVector` (- (`self.SnapPixelToGrid` _returnvalue_x (* (`SceneCaptureComponent2D.OrthoWidth` (`self.SceneCaptureComponent2D`)) (/ 1.0 256.0)) _returnvalue_y) (`self.K2_GetActorLocation`))))
  (bind _output_get (set `self.MoveOffset` (`KismetMathLibrary.MakeVector2D` _returnvalue_x_2 _returnvalue_y_2)))
  (`self.K2_AddActorWorldOffset` (`KismetMathLibrary.MakeVector` (`KismetMathLibrary.BreakVector2D` _output_get) (`.Y` (`KismetMathLibrary.BreakVector2D` _output_get))))
  (`KismetMaterialLibrary.SetVectorParameterValue` "/Game/Blueprints/ReactiveSnow/SnowMPC.SnowMPC" "CaptureLocation" (`KismetMathLibrary.Conv_VectorToLinearColor` (`self.K2_GetActorLocation`))))

(event `DrawToRT`
  (bind _drawtopmat (`self.DrawToPMat`))
  (bind (_returnvalue_x _returnvalue_y) (`KismetMathLibrary.BreakVector2D` (/ (`self.MoveOffset`) (`SceneCaptureComponent2D.OrthoWidth` (`self.SceneCaptureComponent2D`)))))
  (`MaterialInstanceDynamic.SetVectorParameterValue` _drawtopmat "Offset" (make `LinearColor` _returnvalue_x _returnvalue_y 0.0 1.0))
  (`KismetRenderingLibrary.DrawMaterialToRenderTarget` "/Game/Blueprints/ReactiveSnow/RenderTargetPersistent.RenderTargetPersistent" _drawtopmat))

(event `self.ReceiveTick`
  (params (DeltaSeconds :type "Float (single-precision)"))
  (`self.MoveRT`)
  (`self.DrawToRT`))

(fn `UserConstructionScript`)