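; Glowworm burrow (Leuchtwurmbau) light source that starts active or inactive and can be lit by spending 5 of the player's light power.
; Activation toggles the inactive and active lights, then grows the trigger from zero radius to 75% of the active light's attenuation radius.
; Overlapping the trigger marks the player as in a light zone and registers the burrow as interactable, and leaving clears both.
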(event `self.ReceiveBeginPlay`
  ;[1 1 1] Begin Play, Light Intensity Speichern, Zonen setzen
  (if (`self.Inaktiv`)
    (set `self.LightIntensity` (`LightComponentBase.Intensity` (`self.InactiveLight`)))
    (`SceneComponent.SetVisibility` (`self.InactiveLight`) true false)
    (`SceneComponent.SetVisibility` (`self.ActiveLight`) false false)
    (`SphereComponent.SetSphereRadius` (`self.LightTrigger`) 0.0 true)
    (else
      (set `self.LightIntensity` (`LightComponentBase.Intensity` (`self.ActiveLight`)))
      (`SceneComponent.SetVisibility` (`self.InactiveLight`) false false)
      (`SceneComponent.SetVisibility` (`self.ActiveLight`) true false)
      (`SphereComponent.SetSphereRadius` (`self.LightTrigger`) (* (`LocalLightComponent.AttenuationRadius` (`self.ActiveLight`)) 0.75) true))))

(event `Aktivieren`
  ;[1 1 1] Licht Aktivieren
  (bind _asplayer_bp (cast `/Game/ZZZ_TrashCan/PlayerBPs/Player_BP` (`GameplayStatics.GetPlayerCharacter` 0)))
  (bind _currentlightpower (`/Game/ZZZ_TrashCan/PlayerBPs/Player_BP.currentLightPower` _asplayer_bp))
  (if (and (>= _currentlightpower 5.0) (`self.Inaktiv`))
    (set `/Game/ZZZ_TrashCan/PlayerBPs/Player_BP.currentLightPower` (- _currentlightpower 5.0) _asplayer_bp)
    (`SceneComponent.ToggleVisibility` (`self.ActiveLight`) false)
    (`SceneComponent.ToggleVisibility` (`self.InactiveLight`) false)
    (set `self.Inaktiv` false)
    (`SphereComponent.SetSphereRadius` (`self.LightTrigger`) (* (`LocalLightComponent.AttenuationRadius` (`self.ActiveLight`)) 0.75) true)
    (set `self.LightIntensity` (`LightComponentBase.Intensity` (`self.ActiveLight`)))))

(event `self.LightTrigger.OnComponentBeginOverlap`
  (params (OverlappedComponent :type "PrimitiveComponent Object Reference") (OtherActor :type "Actor Object Reference") (OtherComp :type "PrimitiveComponent Object Reference") (OtherBodyIndex :type Integer) (bFromSweep :type Boolean) (SweepResult :type "HitResult Structure (by ref)"))
  ;[1 1 1] Ist Player in der Nähe?
  (bind _asplayer_bp (cast `/Game/ZZZ_TrashCan/PlayerBPs/Player_BP` OtherActor))
  (`/Game/ZZZ_TrashCan/PlayerBPs/Player_BP.SetInteractable` _asplayer_bp self)
  (set `/Game/ZZZ_TrashCan/PlayerBPs/Player_BP.isInLightZone?` true _asplayer_bp))

(event `self.LightTrigger.OnComponentEndOverlap`
  (params (OverlappedComponent :type "PrimitiveComponent Object Reference") (OtherActor :type "Actor Object Reference") (OtherComp :type "PrimitiveComponent Object Reference") (OtherBodyIndex :type Integer))
  ;[1 1 1] Ist Player in der Nähe?
  (bind _asplayer_bp (cast `/Game/ZZZ_TrashCan/PlayerBPs/Player_BP` OtherActor))
  (`/Game/ZZZ_TrashCan/PlayerBPs/Player_BP.ResetInteractable` _asplayer_bp)
  (set `/Game/ZZZ_TrashCan/PlayerBPs/Player_BP.isInLightZone?` false _asplayer_bp))

(fn `UserConstructionScript`)