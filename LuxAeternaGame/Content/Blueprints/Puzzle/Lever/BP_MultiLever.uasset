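; BP_MultiLever is a puzzle lever that starts a target task when interacted with and can reset itself for reuse.
; Interaction calls the parent logic, then a DoOnce gate starts the task, sets a reset timer and rotates the switch via a timeline.
; When the timer expires and Reset is enabled, it stops the task, plays the return rotation and reopens the gate after a short delay.
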(event `self.Interaction`
  ;[1 1 1] Begins the TargetTask sets an End Timer and begins the Animation. (Rotating the lever)
  (`parent.Interaction`)
  (`/Engine/EditorBlueprintResources/StandardMacros.DoOnce` false :!label _label
    (:`Completed`
      (`self.StartTargetTask`)
      (`KismetSystemLibrary.K2_SetTimerDelegate` (delegate `ResetLever`) (`self.ResetTimer`))
      (bind (_direction _yrot) (`Timeline|RotUp` :!via `PlayFromStart`)
        (:`Update`
          (`SceneComponent.K2_SetRelativeRotation` (`self.Switch`) (`KismetMathLibrary.MakeRotator` 0.0 _yrot) false false))))))

(event `ResetLever`
  ;[1 1 1] If bReset? is true: stop the Targets Task play the ResetAnimation and allow further Interaction after a delay.
  (if (`self.bReset?`)
    (`self.StopTargetTask`)
    (bind (_direction _yrot) (`Timeline|RotDown` :!via `PlayFromStart`)
      (:`Update`
        (`SceneComponent.K2_SetRelativeRotation` (`self.Switch`) (`KismetMathLibrary.MakeRotator` 0.0 _yrot) false false))
      (:`Finished`
        (`KismetSystemLibrary.Delay` 0.5)
        (goto _label :!via `Reset`)))))

(fn `UserConstructionScript`)