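; EnemyBox_BP is a damageable enemy box actor that can be destroyed.
; It sets current HP to its maximum on BeginPlay, then subtracts incoming damage through AnyDamage, clamped at zero.
; When HP reaches zero, it destroys itself and plays a sound at its location.
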(event `self.ReceiveBeginPlay`
  (set `self.CurrentHP` (`self.MaxHP`)))

(event `self.ReceiveAnyDamage`
  (params (Damage :type "Float (single-precision)") (DamageType :type "DamageType Object Reference") (InstigatedBy :type "Controller Object Reference") (DamageCauser :type "Actor Object Reference"))
  (bind _output_get (set `self.CurrentHP` (`KismetMathLibrary.FMax` (- (`self.CurrentHP`) Damage))))
  (if (<= _output_get 0.0)
    (`self.K2_DestroyActor`)
    (`GameplayStatics.PlaySoundAtLocation` null (`self.K2_GetActorLocation`) (struct) 1.0 1.0 0.0 null null null)))

(fn `UserConstructionScript`)