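; MinimapCapture is a UI kit actor that sets up a scene capture over a box-shaped area for a minimap.
; Its construction script sizes the box and derives the capture height from box size and field of view, so the view spans the area.
; A valid external map texture sets UseExternalMap and can be displayed on a box-scaled decal through a dynamic material; otherwise the decal is hidden.
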(event EventBeginPlay)

(event EventTick
  (params (DeltaSeconds :type Float%20%28single-precision%29)))

(fn ConstructionScript
  (bind _box_size (Variables|Default|GetBox%20Size))
  (bind _box_size_2 (Variables|Default|GetBox%20Size))
  (Rendering|SetVisibility (Variables|GetMeshComp) false false)
  (Components|Box|SetBoxExtent (Variables|Default|GetBox) (Math|Vector|MakeVector _box_size_2 _box_size_2 2e+01) true)
  (Transformation|SetRelativeLocation (Variables|DecalActor|GetCaptureComponent2D) (Math|Vector|MakeVector 0.0 0.0 (|(x/(tand((f/2)))) (Variables|Default|GetBox%20Size) (Variables|Default|GetField%20Of%20View))) false false)
  (Variables|/Script/Engine.SceneCaptureComponent2D|SetFOVAngle (Variables|DecalActor|GetCaptureComponent2D) (Variables|Default|GetField%20Of%20View))
  (Utilities|IsValid (Variables|Default|GetExternal%20Map)
    (:Is%20Valid
      (Variables|Default|SetUse%20External%20Map true)
      (if (Variables|Default|GetShow%20Decal)
        (bind _returnvalue (Rendering|Material|CreateDynamicMaterialInstance "/Game/UI_Kit/Materials/Misc/M_Decal.M_Decal" "None" :!class /Script/Engine.KismetMaterialLibrary))
        (Rendering|Material|SetTextureParameterValue _returnvalue "texture" (Variables|Default|GetExternal%20Map))
        (Rendering|Components|Decal|SetDecalMaterial (Variables|Default|GetDecal) _returnvalue)
        (Rendering|SetVisibility (Variables|Default|GetDecal) true false)
        (Transformation|SetWorldScale3D (Variables|Default|GetDecal) (Math|Vector|MakeVector _box_size _box_size _box_size))
        (else
          (Rendering|SetVisibility (Variables|Default|GetDecal) false false :!label _label))))
    (:Is%20Not%20Valid
      (Variables|Default|SetUse%20External%20Map false)
      (goto _label))))