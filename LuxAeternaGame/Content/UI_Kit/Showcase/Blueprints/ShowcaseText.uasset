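; Showcase actor that shows a bubble billboard and reveals its text when a Pawn enters its sphere.
; The construction script builds a dynamic bubble material for the billboard and applies the configurable text and sphere radius.
; A timeline fades the bubble out while easing the text's scale and upward movement, reversing on any end overlap.
; Every tick, the text rotates to face the player camera.
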(event `self.ReceiveTick`
  (params (DeltaSeconds :type "Float (single-precision)"))
  (`SceneComponent.K2_SetWorldRotation` (`self.TextRender`) (`KismetMathLibrary.FindLookAtRotation` (`SceneComponent.K2_GetComponentLocation` (`self.TextRender`)) (`self.K2_GetActorLocation` (`GameplayStatics.GetPlayerCameraManager` 0))) false false))

(event `self.Sphere.OnComponentBeginOverlap`
  (params (OverlappedComponent :type "PrimitiveComponent Object Reference") (OtherActor :type "Actor Object Reference") (OtherComp :type "PrimitiveComponent Object Reference") (OtherBodyIndex :type Integer) (bFromSweep :type Boolean) (SweepResult :type "HitResult Structure (by ref)"))
  (bind _returnvalue (enumliteral `EEasingFunc` "EaseIn"))
  (bind _textrender (`self.TextRender`))
  (cast `Pawn` OtherActor)
  (`SceneComponent.SetVisibility` (`self.TextRender`) true false)
  (bind (_direction _percentage) (`Timeline|Text Animation` :!label _label)
    (:`Update`
      (`MaterialInstanceDynamic.SetScalarParameterValue` (`self.Bubble Material`) "Opacity" (- 1.0 _percentage))
      (`SceneComponent.SetWorldScale3D` _textrender (`|EaseFunction` _returnvalue _percentage (0.0 0.0 0.0) (1.0 1.0 1.0)))
      (`SceneComponent.K2_SetRelativeLocation` _textrender (`|EaseFunction` _returnvalue _percentage (0.0 0.0 -50.0)) false false))))

(event `self.Sphere.OnComponentEndOverlap`
  (params (OverlappedComponent :type "PrimitiveComponent Object Reference") (OtherActor :type "Actor Object Reference") (OtherComp :type "PrimitiveComponent Object Reference") (OtherBodyIndex :type Integer))
  (goto _label :!via `Reverse`))

(fn `UserConstructionScript`
  (bind _returnvalue (`KismetMaterialLibrary.CreateDynamicMaterialInstance` "/Game/UI_Kit/Showcase/Materials/M_TextBubble.M_TextBubble"))
  (bind _output_get (set `self.Bubble Material` _returnvalue))
  (`MaterialBillboardComponent.AddElement` (`self.MaterialBillboard`) _output_get null false 32.0 32.0 null)
  (`TextRenderComponent.K2_SetText` (`self.TextRender`) (`self.Text Displayed`))
  (`SphereComponent.SetSphereRadius` (`self.Sphere`) (`self.Sphere Radius`) true))