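; Showcase cube actor for the UI kit that displays an icon texture and periodically animates.
; The construction script puts DisplayedTexture into a dynamic M_IconShowcase material on StaticMesh1 and hides StaticMesh, or applies M_Cube to StaticMesh if no texture is set.
; With a texture, the Movement timeline offsets StaticMesh1 along local X, replaying after random delays so motion recurs at irregular intervals.
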(event `self.ReceiveBeginPlay`
  (`/Engine/EditorBlueprintResources/StandardMacros.IsValid` (`self.Displayed Texture`)
    (:`Is Valid`
      (`KismetSystemLibrary.Delay` (`KismetMathLibrary.RandomFloatInRange` 3.0 15.0))
      (bind (_direction _movement) (`Timeline|Movement`)
        (:`Update`
          (`SceneComponent.K2_SetRelativeLocation` (`self.StaticMesh1`) (`KismetMathLibrary.MakeVector` (* _movement (`self.Offset`))) false false))
        (:`Finished`
          (`KismetSystemLibrary.Delay` (`KismetMathLibrary.RandomFloatInRange` 3.0 15.0))
          (`TimelineComponent.PlayFromStart` (`self.Movement`)))))))

(fn `UserConstructionScript`
  (`/Engine/EditorBlueprintResources/StandardMacros.IsValid` (`self.Displayed Texture`)
    (:`Is Valid`
      (bind _returnvalue (`KismetMaterialLibrary.CreateDynamicMaterialInstance` "/Game/UI_Kit/Showcase/Materials/M_IconShowcase.M_IconShowcase"))
      (`MaterialInstanceDynamic.SetTextureParameterValue` _returnvalue "Icon" (`self.Displayed Texture`))
      (`PrimitiveComponent.SetMaterial` (`self.StaticMesh1`) 1 _returnvalue)
      (`SceneComponent.SetRelativeScale3D` (`self.StaticMesh1`) (0.9 0.9 0.9))
      (`SceneComponent.SetVisibility` (`self.StaticMesh`) false false))
    (:`Is Not Valid`
      (`PrimitiveComponent.SetMaterial` (`self.StaticMesh`) 1 "/Game/UI_Kit/Showcase/Materials/M_Cube.M_Cube"))))