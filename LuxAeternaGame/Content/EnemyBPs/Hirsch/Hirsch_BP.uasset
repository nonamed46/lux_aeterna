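; Hirsch_BP is an enemy actor with health that drops a firefly pickup when killed.
; It starts at MaxHP, subtracts incoming damage clamped at zero, then spawns FireflyPickup_BP at its transform and destroys itself.
; Every tick it writes current HP divided by a fixed 100 to its EnemyHealth widget bar and shows the widget only while the player is within range.
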(event `self.ReceiveBeginPlay`
  ;[1 1 1] Set HP
  (set `self.CurrentHP` (`self.MaxHP`)))

(event `self.ReceiveAnyDamage`
  (params (Damage :type "Float (single-precision)") (DamageType :type "DamageType Object Reference") (InstigatedBy :type "Controller Object Reference") (DamageCauser :type "Actor Object Reference"))
  ;[1 1 1] Receive Damage
  (bind _output_get (set `self.CurrentHP` (`KismetMathLibrary.FMax` (- (`self.CurrentHP`) Damage))))
  (if (<= _output_get 0.0)
    (`|SpawnActorFromClass` "/Game/Blueprints/FireflyPickup_BP.FireflyPickup_BP_C" (`self.GetTransform`) "Undefined" "OverrideRootScale" null null)
    (`self.K2_DestroyActor`)))

(event `self.ReceiveTick`
  (params (DeltaSeconds :type "Float (single-precision)"))
  (bind _returnvalue (`GameplayStatics.GetPlayerCharacter` 0))
  ;[1 1 1] Widget
  (`|ExecutionSequence`
    (:`then_0`
      (bind _asenemy_health (cast `/Game/EnemyBPs/EnemyHealth` (`WidgetComponent.GetUserWidgetObject` (`self.Widget`))))
      (`ProgressBar.SetPercent` (`/Game/EnemyBPs/EnemyHealth.ProgressBar_163` _asenemy_health) (/ (`self.CurrentHP`) 100.0)))
    (:`then_1`
      (`/Engine/EditorBlueprintResources/StandardMacros.IsValid` _returnvalue
        (:`Is Valid`
          (`SceneComponent.SetVisibility` (`self.Widget`) (<= (`KismetMathLibrary.VSize` (- (`self.K2_GetActorLocation` _returnvalue) (`self.K2_GetActorLocation`))) 1000.0) false))))))

(fn `UserConstructionScript`)