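; Stealth component that tracks how lit its owning actor is and picks a priority target from visible actors.
; Lightzone events set illumination, which feeds a light value with base and lantern light; visibility subtracts a cover-level modifier from it.
; Target selection weights each in-range actor's visibility, queried by message, by proximity and flags a target switch.
; GetActorVisibility is a stub returning zero.
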(event `SCEnteredLightzone`
  (params (IlluminationVal :type "Float (double-precision)")))

(event `/Game/Core/Framework/Interfaces/BPI_Stealth.EnterLightzone`
  (params (Luminance :type "Float (single-precision)"))
  (set `self.IlluminationValue` Luminance)
  (set `self.bIlluminated?` true)
  (`KismetSystemLibrary.PrintString` (`KismetStringLibrary.Concat_StrStr` (`KismetSystemLibrary.GetDisplayName` (`self.GetOwner`)) "entered")))

(event `SCExitedLightzone`)

(event `/Game/Core/Framework/Interfaces/BPI_Stealth.ExitLightzone`
  (set `self.IlluminationValue` 0.0)
  (set `self.bIlluminated?` false)
  (`KismetSystemLibrary.PrintString` (`KismetStringLibrary.Concat_StrStr` (`KismetSystemLibrary.GetDisplayName` (`self.GetOwner`)) "exited")))

(fn `CalcLightValue`
  (returns (`new Light Value` :type "Float (double-precision)"))
  (locals (CurrentLightModifiers :type "Float (double-precision)"))
  (`|ExecutionSequence`
    (:`then_0`
      ;[1 1 1] If actor carries a lantern increase the modifier by Lantern Light Value
      (if (`self.bCarryingLantern?`)
        (set `local.CurrentLightModifiers` (+ (`local.CurrentLightModifiers`) (`self.LanternValue`)))))
    (:`then_1`
      ;[1 1 1] If actor is within range of a light source add its illumination value to the modifier
      (if (`self.bIlluminated?`)
        (set `local.CurrentLightModifiers` (+ (`local.CurrentLightModifiers`) (`self.IlluminationValue`)))))
    (:`then_2`
      ;[1 0.7853 0.1129] Calculate and Return the new Current Light Value based on BaseLV and Modifiers
      (bind _output_get (set `self.CurrentLigthValue` (+ (`self.BaseLightValue`) (`local.CurrentLightModifiers`))))
      (return _output_get))))

(fn `CalcVisibility`
  (returns (Visibility :type "Float (double-precision)"))
  ;[1 1 1] Calculates the visibility of an actor by subtracting the "cover modifier value" from the current light value
  (bind _output_get (set `self.Visibility` (- (`self.CurrentLigthValue`) (select `int` (`self.CoverLevel`) :`0` (`self.CoverVal_L0`) :`1` (`self.CoverVal_L1`) :`2` (`self.CoverVal_L2`))))) ; Value Range is 0-100 by default
  (return _output_get))

(fn `GetActorVisibility`
  (returns (Visibility :type "Float (double-precision)"))
  (return 0.0))

(fn `GetPriorityTarget`
  (params (`Current Target` :type "Actor Object Reference") (VisibleTargets :type "Array of Actor Object Reference") (`Aggro Range` :type "Float (double-precision)"))
  (returns (NewPriorityTarget :type "Actor Object Reference") (`(TODO)AttackPriorityList` :type "Array of Actor Object Reference") (`bSwitchTarget?` :type Boolean))
  (locals (L_Target :type "Actor Object Reference") (L_Distance :type "Float (double-precision)") (L_Priority :type "Float (double-precision)"))
  (bind _l_target (`local.L_Target`))
  (set `local.L_Target` `Current Target`)
  ;[1 1 1] component calculates priority list within aggro range based on visibility and distance to target
  (for _array_element VisibleTargets
    ;[1 1 1] If Enemy is valid and in range get its visibility and multiply by the range percentage (further = smaller value). If the calculated priority value is greater than the cached one set this as new target
    (`/Engine/EditorBlueprintResources/StandardMacros.IsValid` _array_element
      (:`Is Valid`
        (bind (_returnvalue _distance _aggro_range_pt_) (`self.isValidEnemyInRange?` _array_element `Aggro Range`))
        (if _returnvalue
          (bind _output_get (set `local.L_Distance` _distance))
          (bind _visibility (message `/Game/Core/Framework/Interfaces/BPI_Stealth.GetActorVisibility` _array_element))
          (bind _returnvalue_2 (* _visibility (- 1.0 (/ _output_get _aggro_range_pt_))))
          (if (> _returnvalue_2 (`local.L_Priority`))
            (set `local.L_Priority` _returnvalue_2)
            (set `local.L_Target` _array_element))))))
  ;[1 1 1] Returns priority list, new priority target and bool if it needs to switch targets
  (return _l_target _ (!= _l_target `Current Target`)))