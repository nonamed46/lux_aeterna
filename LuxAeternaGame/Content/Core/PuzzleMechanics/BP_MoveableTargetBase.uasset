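; Base puzzle target that moves a mesh between two transforms when its task starts, using a timeline with configurable length and optional curve override.
; Stopping the task halts, reverses after a delay or continues the movement, based on ReverseState.
; With Reset enabled, a finished move returns from the end after a delay, while a gate blocks stop-triggered reversals until the return completes.
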(event `self.ReceiveBeginPlay`
  (bind _movementcurve (`self.MovementCurve`))
  ;[1 1 1] On BeginPlay if MovementCurve Variable is valid, set it as new Float Curve
  (`/Engine/EditorBlueprintResources/StandardMacros.IsValid` _movementcurve
    (:`Is Valid`
      (`TimelineComponent.SetFloatCurve` (`self.Movement`) _movementcurve "TransformAlpha"))))

(event `self.StartTask`
  (bind (_direction _transformalpha) (`Timeline|Movement` :!label _label)
    (:`Update`
      (`SceneComponent.K2_SetWorldTransform` (`self.MovingMesh`) (`self.Lerp_A-B_Transform` _transformalpha) false false))
    (:`Finished`
      (if (`self.bReset?`)
        (`KismetSystemLibrary.K2_SetTimerDelegate` (delegate `ResetMovement`) (`self.ResetDelay`)) ; Reverses From End after Delay to reset to original Position
        (goto _label_2 :!via `Close`)))))

(event `self.StopTask`
  ;[1 1 1] STOP TASK: Chooses between Stopping, Reversing or Continuing the Movement
  (switch `/Game/Core/Framework/ENUMS/E_PuzzleTargetReverse` (`self.ReverseState`)
    (:`NewEnumerator1`
      (goto _label :!via `Stop`))
    (:`NewEnumerator2`
      (`KismetSystemLibrary.K2_SetTimerDelegate` (delegate `ReverseMovement`) (`self.ReverseDelay`)) ; Reverse after Delay
    )))

(event `ReverseMovement`
  (`/Engine/EditorBlueprintResources/StandardMacros.Gate` true :!label _label_2
    (:`Exit`
      (goto _label :!via `Reverse`))))

(event `ResetMovement`
  (`|ExecutionSequence`
    (:`then_0`
      (goto _label :!via `ReverseFromEnd`))
    (:`then_1`
      (`KismetSystemLibrary.Delay` (`TimelineComponent.GetTimelineLength` (`self.Movement`)))
      (goto _label_2 :!via `Open`))))

(fn `UserConstructionScript`
  (`parent.UserConstructionScript`)
  (`TimelineComponent.SetTimelineLength` (`self.Movement`) (`self.MovementLength`)))