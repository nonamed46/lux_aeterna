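; Base puzzle-mechanic actor that spins a mesh through a RotatingMovement component in response to task start and stop events.
; StartTask activates rotation after a delay, while StopTask deactivates it after its own delay only if the Deactivate flag is set.
; The construction script offsets the mesh and applies rotation speed, pivot and start-rotating settings.
; Overlapping ALS characters receive a slight radial impulse on their mesh.
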(event `self.StartTask`
  (`KismetSystemLibrary.K2_SetTimerDelegate` (delegate `Activate`) (`self.ActivationDelay`))
  (`KismetSystemLibrary.PrintString` "Activation started"))

(event `Activate`
  (`ActorComponent.Activate` (`self.RotatingMovement`) false)
  (`KismetSystemLibrary.PrintString` "activated"))

(event `self.StopTask`
  (if (`self.bDeactivate?`)
    (`KismetSystemLibrary.K2_SetTimerDelegate` (delegate `Deactivate`) (`self.DeactivationDelay`))))

(event `Deactivate`
  (`ActorComponent.Deactivate` (`self.RotatingMovement`)))

(event `self.StaticMesh.OnComponentBeginOverlap`
  (params (OverlappedComponent :type "PrimitiveComponent Object Reference") (OtherActor :type "Actor Object Reference") (OtherComp :type "PrimitiveComponent Object Reference") (OtherBodyIndex :type Integer) (bFromSweep :type Boolean) (SweepResult :type "HitResult Structure (by ref)"))
  (bind _asals_base_character (cast `/Game/Core/Characters/AdvancedLocomotionV3/Blueprints/ALS_BaseCharacter` OtherActor))
  (`PrimitiveComponent.AddRadialImpulse` (`Character.Mesh` _asals_base_character) (0.0 0.0 0.0) 50.0 0.1 "RIF_Constant" true))

(fn `UserConstructionScript`
  (bind _staticmesh (`self.StaticMesh`))
  (bind _rotatingmovement (`self.RotatingMovement`))
  (`parent.UserConstructionScript`)
  ;[1 1 1] Offset Rotating Mesh
  (`SceneComponent.K2_SetWorldLocation` _staticmesh (+ (`SceneComponent.K2_GetComponentLocation` _staticmesh) (`self.RotatingMeshOffset`)) false false)
  ;[1 1 1] Set Rotating Movement Speed and Pivot Translation (Offset)
  (set `RotatingMovementComponent.RotationRate` (`self.RotationSpeed`) _rotatingmovement)
  (set `RotatingMovementComponent.PivotTranslation` (`self.RotationPivotTranslation`) _rotatingmovement)
  (`ActorComponent.SetAutoActivate` _rotatingmovement (`self.bRotateOnStart?`)))