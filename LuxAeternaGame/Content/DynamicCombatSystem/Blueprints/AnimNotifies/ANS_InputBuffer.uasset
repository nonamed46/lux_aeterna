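; Anim notify state that marks the window in an animation during which input buffering is open.
; On begin it finds the owner's InputBufferComponent and opens the buffer, and on end it closes it.
; It does nothing if the owner has no such component, and it shows as "InpBuffer" on the animation timeline.
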(fn `GetNotifyName`
  (returns (ReturnValue :type String))
  (return "InpBuffer"))

(fn `Received_NotifyBegin`
  (params (MeshComp :type "SkeletalMeshComponent Object Reference") (Animation :type "AnimSequenceBase Object Reference") (TotalDuration :type "Float (double-precision)"))
  (returns (ReturnValue :type Boolean))
  (bind _returnvalue (`Actor.GetComponentByClass` (`ActorComponent.GetOwner` MeshComp) "/Game/DynamicCombatSystem/Blueprints/Components/InputBufferComponent.InputBufferComponent_C"))
  (`/Engine/EditorBlueprintResources/StandardMacros.IsValid` _returnvalue
    (:`Is Valid`
      (`/Game/DynamicCombatSystem/Blueprints/Components/InputBufferComponent.OpenInputBuffer` _returnvalue)
      (return false))))

(fn `Received_NotifyEnd`
  (params (MeshComp :type "SkeletalMeshComponent Object Reference") (Animation :type "AnimSequenceBase Object Reference"))
  (returns (ReturnValue :type Boolean))
  (bind _returnvalue (`Actor.GetComponentByClass` (`ActorComponent.GetOwner` MeshComp) "/Game/DynamicCombatSystem/Blueprints/Components/InputBufferComponent.InputBufferComponent_C"))
  (`/Engine/EditorBlueprintResources/StandardMacros.IsValid` _returnvalue
    (:`Is Valid`
      (`/Game/DynamicCombatSystem/Blueprints/Components/InputBufferComponent.CloseInputBuffer` _returnvalue)
      (return false))))